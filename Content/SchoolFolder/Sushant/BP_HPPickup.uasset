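; BP_HPPickup is a pickup that raises the Deaths counter on SideScrollerGameMode when the player character touches it.
; On box overlap it finds the game mode through GetAllActorsOfClass and, while Deaths is below 3, increments it, prints it and destroys itself.
; At 3 or more the pickup stays in the world.
; Tick calls BeginTrails on its particle system every frame.
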(event `self.ReceiveTick`
  (params (DeltaSeconds :type "Float (single-precision)"))
  (`ParticleSystemComponent.BeginTrails` (`self.ParticleSystem`) "None" "None" "ETrailWidthMode_FromCentre" 0.0))

(event `self.Box.OnComponentBeginOverlap`
  (params (OverlappedComponent :type "PrimitiveComponent Object Reference") (OtherActor :type "Actor Object Reference") (OtherComp :type "PrimitiveComponent Object Reference") (OtherBodyIndex :type Integer) (bFromSweep :type Boolean) (SweepResult :type "HitResult Structure (by ref)"))
  (if (== (`GameplayStatics.GetPlayerCharacter` 0) OtherActor)
    (bind _outactors (`GameplayStatics.GetAllActorsOfClass` "/Game/SideScrollerBP/Blueprints/SideScrollerGameMode.SideScrollerGameMode_C"))
    (bind _output_get (set `self.gamemoderef` (`|GetArrayItem` _outactors)))
    (bind _deaths (`/Game/SideScrollerBP/Blueprints/SideScrollerGameMode.deaths` _output_get))
    (if (not (>= _deaths 3))
      (bind _result (`/Engine/EditorBlueprintResources/StandardMacros.IncrementInt` _deaths)
        (:`  `
          (set `/Game/SideScrollerBP/Blueprints/SideScrollerGameMode.deaths` _result _output_get)
          (`KismetSystemLibrary.PrintString` (`KismetStringLibrary.Conv_IntToString` _deaths))
          (`self.K2_DestroyActor`))))))

(fn `UserConstructionScript`)