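; Checkpoint actor that updates the player's spawn point in the side-scroller when touched.
; The first Box overlap passes a DoOnce; if it is player 0, the Arrow's location, without rotation, becomes SpawnTransform on the SideScrollerGameMode, then is printed.
; The DoOnce precedes the player check, so any other overlapping actor uses up the checkpoint.
; The game mode is found via GetAllActorsOfClass; CastingToCharacter is an empty stub.
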(event `self.Box.OnComponentBeginOverlap`
  (params (OverlappedComponent :type "PrimitiveComponent Object Reference") (OtherActor :type "Actor Object Reference") (OtherComp :type "PrimitiveComponent Object Reference") (OtherBodyIndex :type Integer) (bFromSweep :type Boolean) (SweepResult :type "HitResult Structure (by ref)"))
  (`/Engine/EditorBlueprintResources/StandardMacros.DoOnce` false
    (:`Completed`
      (if (== OtherActor (`GameplayStatics.GetPlayerCharacter` 0))
        (bind _outactors (`GameplayStatics.GetAllActorsOfClass` "/Game/SideScrollerBP/Blueprints/SideScrollerGameMode.SideScrollerGameMode_C"))
        (bind _output_get (set `self.GamemodeRef` (`|GetArrayItem` _outactors)))
        (bind _output_get_2 (set `/Game/SideScrollerBP/Blueprints/SideScrollerGameMode.Spawn Transform` (`KismetMathLibrary.Conv_VectorToTransform` (`SceneComponent.K2_GetComponentLocation` (`self.Arrow`))) _output_get))
        (`KismetSystemLibrary.PrintString` (`KismetStringLibrary.Conv_TransformToString` _output_get_2))))))

(fn `CastingToCharacter`
  (params (A :type "Object Object Reference"))
  (if (== A (`GameplayStatics.GetPlayerCharacter` 0))
    _))

(fn `UserConstructionScript`)