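; BP_boulder1 is a boulder hazard pawn that travels across the level and reacts to hitting the player.
; On BeginPlay it halves its mesh scale and uses AI MoveTo toward the first TargetPoint found in the level, destroying itself on arrival.
; Overlap of its Sphere with the player character prints a hit message and destroys the boulder, with no damage applied.
; A separate Destroy event also removes it.
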(event `self.ReceiveBeginPlay`
  (`|ExecutionSequence`
    (:`then_0`
      (bind _outactors (`GameplayStatics.GetAllActorsOfClass` "/Script/Engine.TargetPoint"))
      (`|AIMoveTo` self (0.0 0.0 0.0) (`|GetArrayItem` _outactors)
        (:`OnSuccess`
          (`self.K2_DestroyActor`))))
    (:`then_1`
      (`SceneComponent.SetWorldScale3D` (`self.StaticMesh`) (0.5 0.5 0.5)))))

(event `self.Sphere.OnComponentBeginOverlap`
  (params (OverlappedComponent :type "PrimitiveComponent Object Reference") (OtherActor :type "Actor Object Reference") (OtherComp :type "PrimitiveComponent Object Reference") (OtherBodyIndex :type Integer) (bFromSweep :type Boolean) (SweepResult :type "HitResult Structure (by ref)"))
  (if (== OtherActor (`GameplayStatics.GetPlayerCharacter` 0))
    (`KismetSystemLibrary.PrintString` "you got hit")
    (`self.K2_DestroyActor`)))

(event `/Game/SchoolFolder/Sushant/INT_AI.Destroy`
  (`self.K2_DestroyActor`))

(fn `UserConstructionScript`)