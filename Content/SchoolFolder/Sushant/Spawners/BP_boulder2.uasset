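; BP_boulder2 is a boulder hazard pawn that travels to a despawn point and destroys the player character on contact.
; On BeginPlay it takes the first BP_despawn actor it finds as its AI move target, destroying itself when the move succeeds.
; It also sets the world scale of its static mesh from Scaleparams.
; A sphere overlap with the player character destroys that character outright.
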(event `self.ReceiveBeginPlay`
  (`|ExecutionSequence`
    (:`then_0`
      (bind _outactors (`GameplayStatics.GetAllActorsOfClass` "/Game/SchoolFolder/Sushant/Spawners/BP_despawn.BP_despawn_C"))
      (bind _output_get (set `self.DespawnerRef` (`|GetArrayItem` _outactors)))
      (`|AIMoveTo` self (0.0 0.0 0.0) _output_get
        (:`OnSuccess`
          (`self.K2_DestroyActor`))))
    (:`then_1`
      (`SceneComponent.SetWorldScale3D` (`self.StaticMesh`) (`self.Scaleparams`)))))

(event `self.Sphere.OnComponentBeginOverlap`
  (params (OverlappedComponent :type "PrimitiveComponent Object Reference") (OtherActor :type "Actor Object Reference") (OtherComp :type "PrimitiveComponent Object Reference") (OtherBodyIndex :type Integer) (bFromSweep :type Boolean) (SweepResult :type "HitResult Structure (by ref)"))
  (bind _returnvalue (`GameplayStatics.GetPlayerCharacter` 0))
  (if (== OtherActor _returnvalue)
    (`self.K2_DestroyActor` _returnvalue)))

(fn `UserConstructionScript`)